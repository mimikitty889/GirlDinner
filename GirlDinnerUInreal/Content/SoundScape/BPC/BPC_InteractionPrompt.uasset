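; Actor component that shows a screen-space interaction prompt while something overlaps its owner's sphere collision.
; On BeginPlay it creates a WB_InteractionPrompt widget with the configured display text and hosts it in a hidden WidgetComponent added at the owner's ArrowComponent relative transform.
; The owner's SphereComponent begin and end overlap events toggle the prompt's visibility, with no filter on the overlapping actor.
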(event Custom|EventBeginOverlap
  (params (OverlappedComponent :type Primitive%20Component%20Object%20Reference) (OtherActor :type Actor%20Object%20Reference) (OtherComp :type Primitive%20Component%20Object%20Reference) (OtherBodyIndex :type Integer) (bFromSweep :type Boolean) (SweepResult :type Hit%20Result%20Structure%20%28by%20ref%29))
  (Rendering|SetVisibility (Variables|Reference|GetRef_WidgetComponent) true false))

(event Custom|EventEndOverlap
  (params (OverlappedComponent :type Primitive%20Component%20Object%20Reference) (OtherActor :type Actor%20Object%20Reference) (OtherComp :type Primitive%20Component%20Object%20Reference) (OtherBodyIndex :type Integer))
  (Rendering|SetVisibility (Variables|Reference|GetRef_WidgetComponent) false false))

(event EventBeginPlay
  (bind _returnvalue (Components|GetOwner))
  (bind _returnvalue_2 (UserInterface|CreateWidget "/Game/SoundScape/Interface/WB_InteractionPrompt.WB_InteractionPrompt_C"))
  (Variables|Reference|SetRefWidget _returnvalue_2)
  (Default|EventChangeTexte (Variables|Reference|GetRefWidget) (Variables|Default|GetDisplayString))
  (Variables|Reference|SetRef_SphereCollision (Actor|GetComponentbyClass (Components|GetOwner) "/Script/Engine.SphereComponent"))
  (bind _returnvalue_3 (Game|AddComponentbyClass _returnvalue "/Script/UMG.WidgetComponent" false (Transformation|GetRelativeTransform (Actor|GetComponentbyClass _returnvalue "/Script/Engine.ArrowComponent"))))
  (Variables|Reference|SetRef_WidgetComponent _returnvalue_3)
  (Class|WidgetComponent|SetWidgetSpace (Variables|Reference|GetRef_WidgetComponent) "Screen")
  (Rendering|SetVisibility (Variables|Reference|GetRef_WidgetComponent) false false)
  (UserInterface|SetWidget (Variables|Reference|GetRef_WidgetComponent) (Variables|Reference|GetRefWidget))
  (Collision|BindEventtoOnComponentBeginOverlap (Variables|Reference|GetRef_SphereCollision) (delegate Custom|EventBeginOverlap))
  (Collision|BindEventtoOnComponentEndOverlap (Variables|Reference|GetRef_SphereCollision) (delegate Custom|EventEndOverlap)))